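; World floor that sets up the agent simulation for the GameMode's TreeType: None, Quadtree or Octree.
; BeginPlay scales the cube, builds the placed tree actor from its bounds and OctreeHeight, then spawns agents at random points.
; Tree modes hand the agent list to the tree, while None gives each agent all others and builds the octree only for C++ bounds.
; PopulateTree, a distance-colored query visualization, is called only from disconnected nodes.
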(event EventBeginPlay
  (bind _cube (Variables|Default|GetCube))
  (bind _allagents (Variables|Default|GetAllAgents))
  (bind _octreeheight (Variables|Default|GetOctreeHeight))
  (bind _box (Variables|Default|GetBox))
  (bind _octreeheight_2 (Variables|Default|GetOctreeHeight))
  (bind _box_2 (Variables|Default|GetBox))
  (bind _octreeheight_3 (Variables|Default|GetOctreeHeight))
  (bind _octreeheight_4 (Variables|Default|GetOctreeHeight))
  (bind _box_3 (Variables|Default|GetBox))
  (bind (_origin _boxextent) (Collision|GetComponentBounds _cube))
  (bind _returnvalue (Components|Box|GetScaledBoxExtent _box))
  (bind _returnvalue_2 (Components|Box|GetScaledBoxExtent _box_3))
  (bind _returnvalue_3 (Components|Box|GetScaledBoxExtent _box_2))
  (bind _returnvalue_4 (* _octreeheight 0.5))
  (bind _returnvalue_5 (* _octreeheight_2 0.5))
  (bind _returnvalue_6 (* _octreeheight_4 0.5))
  (bind _returnvalue_7 (- (.x _origin) (.x _boxextent)))
  (bind _returnvalue_8 (- (.y _origin) (.y _boxextent)))
  (bind _returnvalue_9 (+ (.x _origin) (.x _boxextent)))
  (bind _returnvalue_10 (+ (.y _origin) (.y _boxextent)))
  (bind _returnvalue_11 (Math|Vector|MakeVector _returnvalue_7 _returnvalue_8 (.z _origin)))
  (bind _returnvalue_12 (Math|Vector|MakeVector _returnvalue_9 _returnvalue_10 _octreeheight_3))
  (Transformation|SetWorldScale3D _cube (Variables|Default|GetScaleOnStart))
  (bind _asbp_game_mode (Utilities|Casting|CastToBP_GameMode (Game|GetGameMode)))
  (Utilities|FlowControl|DelayUntilNextTick)
  (switch Utilities|FlowControl|Switch|SwitchonETreeType (Variables|/Script/Gradwork.GradworkGameMode|GettreeType _asbp_game_mode)
    (:none
      (bind _returnvalue_13 (Actor|GetActorOfClass "/Game/Project/BP_Octree.BP_Octree_C"))
      (bind _output_get (Variables|Default|SetOctree _returnvalue_13))
      ;[1 1 1] we build the octree here just for its bounds which gets accessed in cpp.
      (Class|Octree|Build _output_get (Math|Box|MakeBox _returnvalue_11 _returnvalue_12))
      (for _index (range 0 (- (Variables|Default|GetAmountActors) 1))
        (bind _returnvalue_14 (Game|SpawnActorfromClass "/Game/Project/BP_Agent.BP_Agent_C" (Math|Conversions|ToTransform(Vector) (Math|Random|RandomPointinBoundingBox (Math|Vector|MakeVector 0.0 0.0 _returnvalue_4) (Math|Vector|MakeVector (.x _returnvalue) (.y _returnvalue) _returnvalue_4))) "Undefined" "MultiplyWithRoot" 0 0))
        (Utilities|Array|AddUnique (Variables|Default|GetAllAgents) _returnvalue_14))
      (for _array_element _allagents
        (bind _output_get_2 (Variables|/Script/Gradwork.Agent|SetOtherActors _array_element _allagents))
        ;[1 1 1] remove itself from the array
        (Utilities|Array|RemoveItem _output_get_2 _array_element)))
    (:quadtree
      ;[1 1 1] Quadtree
      (bind _returnvalue_15 (Actor|GetActorOfClass "/Game/Project/BP_QuadTree.BP_QuadTree_C"))
      (bind _output_get_3 (Variables|Default|SetQuadTree _returnvalue_15))
      (Class|QuadTree|Build _output_get_3 (Math|Box|MakeBox _returnvalue_11 _returnvalue_12))
      (Utilities|FlowControl|Delay 2.0)
      (for _index_2 (range 0 (- (Variables|Default|GetAmountActors) 1))
        (bind _returnvalue_16 (Game|SpawnActorfromClass "/Game/Project/BP_Agent.BP_Agent_C" (Math|Conversions|ToTransform(Vector) (Math|Random|RandomPointinBoundingBox (Math|Vector|MakeVector 0.0 0.0 _returnvalue_6) (Math|Vector|MakeVector (.x _returnvalue_2) (.y _returnvalue_2) _returnvalue_6))) "Undefined" "MultiplyWithRoot" 0 0))
        (Utilities|Array|AddUnique (Variables|Default|GetAllAgents) _returnvalue_16))
      (Variables|/Script/Gradwork.QuadTree|SetallActors (Variables|Default|GetQuadTree) (Variables|Default|GetAllAgents)))
    (:octree
      ;[1 1 1] Octree
      (bind _returnvalue_17 (Actor|GetActorOfClass "/Game/Project/BP_Octree.BP_Octree_C"))
      (bind _output_get_4 (Variables|Default|SetOctree _returnvalue_17))
      (Class|Octree|Build _output_get_4 (Math|Box|MakeBox _returnvalue_11 _returnvalue_12))
      (for _index_3 (range 0 (- (Variables|Default|GetAmountActors) 1))
        (bind _returnvalue_18 (Game|SpawnActorfromClass "/Game/Project/BP_Agent.BP_Agent_C" (Math|Conversions|ToTransform(Vector) (Math|Random|RandomPointinBoundingBox (Math|Vector|MakeVector 0.0 0.0 _returnvalue_5) (Math|Vector|MakeVector (.x _returnvalue_3) (.y _returnvalue_3) _returnvalue_5))) "Undefined" "MultiplyWithRoot" 0 0))
        (Utilities|Array|AddUnique (Variables|Default|GetAllAgents) _returnvalue_18))
      (Variables|/Script/Gradwork.Octree|SetallActors (Variables|Default|GetOctree) (Variables|Default|GetAllAgents)))))

(event Collision|EventActorBeginOverlap
  (params (OtherActor :type Actor%20Object%20Reference)))

(event EventTick
  (params (DeltaSeconds :type Float%20%28single-precision%29))
  ;[1 1 1] Octree
)

(fn ConstructionScript)

(fn PopulateTree
  (bind _amountactors (Variables|Default|GetAmountActors))
  (bind _output_get (Variables|Default|SetRandomIndex (Math|Random|RandomInteger _amountactors)))
  (for _index (range 0 (- _amountactors 1))
    (bind _returnvalue (Game|SpawnActorfromClass "/Game/Project/BP_Agent.BP_Agent_C" (Math|Conversions|ToTransform(Vector) (Math|Random|RandomPointinBoundingBox (Math|Vector|MakeVector 0.0 0.0 (.z (.location (Transformation|GetActorTransform (Variables|Default|GetQuadTree))))) (Components|Box|GetScaledBoxExtent (Variables|Default|GetBox)))) "AdjustIfPossibleButAlwaysSpawn" "MultiplyWithRoot" 0 0))
    (Utilities|Array|AddUnique (Variables|Default|GetAllAgents) _returnvalue)
    (Class|Octree|Insert (Variables|Default|GetOctree) _returnvalue))
  (Variables|Default|SetchosenAgent (Utilities|Array|Get(acopy) (Variables|Default|GetAllAgents) _output_get))
  (Rendering|Material|SetMaterial (Variables|/Game/Project/BP_Agent.BP_Agent_C|GetSphere (Utilities|Array|Get(acopy) (Variables|Default|GetAllAgents) _output_get)) 0 "/Game/Project/Materials/M_ChosenAgent.M_ChosenAgent")
  (Class|Agent|QueryTree (Utilities|Array|Get(acopy) (Variables|Default|GetAllAgents) _output_get))
  (for _array_element (Variables|/Script/Gradwork.Agent|GetOtherActors (Utilities|Array|Get(acopy) (Variables|Default|GetAllAgents) _output_get))
    (bind _returnvalue_2 (Rendering|Material|CreateDynamicMaterialInstance "/Game/Project/Materials/MI_ChosenAgent.MI_ChosenAgent" "None" "None" :!class /Script/Engine.KismetMaterialLibrary))
    (bind _asbp_agent (Utilities|Casting|CastToBP_Agent _array_element))
    (Rendering|Material|SetVectorParameterValue _returnvalue_2 "Color" (Math|Conversions|ToLinearColor(Vector) (Math|Vector|Lerp(Vector) (Math|Conversions|ToVector(LinearColor) "(R=0.069925,G=1.000000,B=0.000000,A=1.000000)") (Math|Conversions|ToVector(LinearColor) (LocalVariables|GetColor)) (/ (Class|KismetMathLibrary|DistanceSquared2D (Math|Conversions|ToVector2D(Vector) (Transformation|GetActorLocation _asbp_agent)) (Math|Conversions|ToVector2D(Vector) (Transformation|GetActorLocation (Utilities|Array|Get(acopy) (Variables|Default|GetAllAgents) _output_get)))) 5e+05))) :!class /Script/Engine.MaterialInstanceDynamic)
    (Rendering|Material|SetMaterial (Variables|/Game/Project/BP_Agent.BP_Agent_C|GetSphere _asbp_agent) 0 _returnvalue_2)))